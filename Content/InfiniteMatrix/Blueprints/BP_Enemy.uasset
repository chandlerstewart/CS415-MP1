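; BP_Enemy is an enemy actor that destroys itself the first time its BoxCollider overlaps another actor.
; A BP_Player hit loses 30 health, capped at MaxHealth and truncated to a whole number, and at zero or below is marked dead and shown the restart display.
; Any other overlapping actor makes every BP_Player in the level gain 2 score, with no check on what that actor is.
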(event OnComponentBeginOverlap(BoxCollider)
  (params (OverlappedComponent :type Primitive%20Component%20Object%20Reference) (OtherActor :type Actor%20Object%20Reference) (OtherComp :type Primitive%20Component%20Object%20Reference) (OtherBodyIndex :type Integer) (bFromSweep :type Boolean) (SweepResult :type Hit%20Result%20Structure%20%28by%20ref%29))
  (Utilities|FlowControl|Sequence
    (:then_0
      (if (Utilities|ClassIsChildOf (Utilities|GetClass OtherActor) "/Game/InfiniteMatrix/Blueprints/BP_Player.BP_Player_C")
        (bind _asbp_player (Utilities|Casting|CastToBP_Player OtherActor))
        (bind _output_get (Variables|/Game/InfiniteMatrix/Blueprints/BP_Player.BP_Player_C|SetHealth _asbp_player (Math|Conversions|ToFloat(Integer) (Class|KismetMathLibrary|MinInt64 (Class|KismetMathLibrary|ToInt64(Float) (- (Variables|/Game/InfiniteMatrix/Blueprints/BP_Player.BP_Player_C|GetHealth _asbp_player) 3e+01)) (Class|KismetMathLibrary|ToInt64(Float) (Variables|/Game/InfiniteMatrix/Blueprints/BP_Player.BP_Player_C|GetMaxHealth _asbp_player))))))
        (if (<= _output_get 0.0)
          (Variables|/Game/InfiniteMatrix/Blueprints/BP_Player.BP_Player_C|SetIsDead _asbp_player true)
          (Default|DisplayRestart _asbp_player))
        (else
          (bind _outactors (Actor|GetAllActorsOfClass "/Game/InfiniteMatrix/Blueprints/BP_Player.BP_Player_C"))
          (Default|AddtoScore _outactors 2))))
    (:then_1
      (Actor|DestroyActor))))

(event EventBeginPlay)

(event Collision|EventActorBeginOverlap
  (params (OtherActor :type Actor%20Object%20Reference)))

(event EventTick
  (params (DeltaSeconds :type Float%20%28single-precision%29)))

(fn ConstructionScript)