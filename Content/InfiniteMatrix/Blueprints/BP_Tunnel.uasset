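; BP_Tunnel is a tunnel segment with a rotating holed wall that the player passes through to score.
; Its trigger has TunnelSpawner spawn the next tunnel, health pack and enemies, awards a point and destroys this segment.
; Wall hits damage the player, costing a point or triggering death and restart, and destroy other actors.
; Helper functions randomize wall mesh and roll, and tint a dynamic material green-to-red by score.
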(event OnComponentBeginOverlap(TriggerZone)
  (params (OverlappedComponent :type Primitive%20Component%20Object%20Reference) (OtherActor :type Actor%20Object%20Reference) (OtherComp :type Primitive%20Component%20Object%20Reference) (OtherBodyIndex :type Integer) (bFromSweep :type Boolean) (SweepResult :type Hit%20Result%20Structure%20%28by%20ref%29))
  (bind _tunnelspawner (Variables|Default|GetTunnelSpawner))
  (bind _newesttunnel (Variables|/Game/InfiniteMatrix/Blueprints/BP_TunnelSpawner.BP_TunnelSpawner_C|GetNewestTunnel _tunnelspawner))
  (if (Utilities|ClassIsChildOf (Utilities|GetClass OtherActor) "/Game/InfiniteMatrix/Blueprints/BP_Player.BP_Player_C")
    (Utilities|FlowControl|Sequence
      (:then_0
        (bind _asbp_player (Utilities|Casting|CastToBP_Player OtherActor))
        (Default|SpawnTunnelatSpawnPoint (Variables|Default|GetTunnelSpawner))
        (Default|AddtoScore _asbp_player 1)
        (Actor|DestroyActor))
      (:then_1
        (Default|SpawnHealthPack _tunnelspawner _newesttunnel)
        (Default|SpawnEnemies _tunnelspawner _newesttunnel)))))

(event OnComponentBeginOverlap(WallMesh)
  (params (OverlappedComponent :type Primitive%20Component%20Object%20Reference) (OtherActor :type Actor%20Object%20Reference) (OtherComp :type Primitive%20Component%20Object%20Reference) (OtherBodyIndex :type Integer) (bFromSweep :type Boolean) (SweepResult :type Hit%20Result%20Structure%20%28by%20ref%29))
  (if (Utilities|ClassIsChildOf (Utilities|GetClass OtherActor) "/Game/InfiniteMatrix/Blueprints/BP_Player.BP_Player_C")
    (bind _asbp_player (Utilities|Casting|CastToBP_Player OtherActor))
    (bind _output_get (Variables|/Game/InfiniteMatrix/Blueprints/BP_Player.BP_Player_C|SetHealth _asbp_player (- (Variables|/Game/InfiniteMatrix/Blueprints/BP_Player.BP_Player_C|GetHealth _asbp_player) 25.0)))
    (if (<= _output_get 0.0)
      (Variables|/Game/InfiniteMatrix/Blueprints/BP_Player.BP_Player_C|SetIsDead _asbp_player true)
      (Default|DisplayRestart _asbp_player)
      (else
        (Utilities|FlowControl|Sequence
          (:then_0
            (Collision|SetCollisionEnabled (Variables|Default|GetWallMesh) "NoCollision"))
          (:then_1
            (Variables|/Game/InfiniteMatrix/Blueprints/BP_Player.BP_Player_C|SetScore _asbp_player (- (Variables|/Game/InfiniteMatrix/Blueprints/BP_Player.BP_Player_C|GetScore _asbp_player) 1))))))
    (else
      (Actor|DestroyActor OtherActor))))

(event EventTick
  (params (DeltaSeconds :type Float%20%28single-precision%29))
  (Transformation|AddLocalRotation (Variables|Default|GetWallMesh) (Math|Rotator|MakeRotator (* DeltaSeconds (Variables|Default|GetRotateSpeed)) 0.0 0.0) false false))

(fn ConstructionScript)

(fn RandomizeWall
  (Components|StaticMesh|SetStaticMesh (Variables|Default|GetWallMesh) (Utilities|Select :Index (Math|Random|RandomIntegerinRange 0 3) :Option%200 "/Game/InfiniteMatrix/Meshes/SM_Hole_01.SM_Hole_01" :Option%201 "/Game/InfiniteMatrix/Meshes/SM_Hole_02.SM_Hole_02" :Option%202 "/Game/InfiniteMatrix/Meshes/SM_Hole_03.SM_Hole_03" :Option%203 "/Game/InfiniteMatrix/Meshes/SM_Hole_04.SM_Hole_04"))
  (Transformation|AddLocalRotation (Variables|Default|GetWallMesh) (Math|Rotator|MakeRotator (Math|Random|RandomFloatinRange 0.0 3.6e+02) 0.0 0.0) false false))

(fn ChangeColor
  (bind _returnvalue (Rendering|Material|CreateDynamicMaterialInstance (Variables|Debug|GetStaticMeshComponent) 0 0 "None" :!class /Script/Engine.PrimitiveComponent))
  (bind _outactors (Actor|GetAllActorsOfClass "/Game/InfiniteMatrix/Blueprints/BP_Player.BP_Player_C"))
  (for _array_element _outactors
    (Rendering|Material|SetVectorParameterValue _returnvalue "BackgroundColor" (Math|Color|Lerp(LinearColor) (Utilities|Struct|MakeLinearColor 0.0 1.0 0.0 0.8) (Utilities|Struct|MakeLinearColor 1.0 0.0 0.0 0.8) (Math|Float|SafeDivide (Math|Conversions|ToFloat(Integer) (Variables|/Game/InfiniteMatrix/Blueprints/BP_Player.BP_Player_C|GetScore _array_element)) 1e+02)) :!class /Script/Engine.MaterialInstanceDynamic)))